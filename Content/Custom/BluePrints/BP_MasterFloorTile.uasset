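; BP_MasterFloorTile is a floor tile for an endless-runner level with three lanes.
; On BeginPlay it spawns an actor, intended as an obstacle, at a randomly chosen lane transform.
; When its Box trigger is overlapped, it tells ThirdPersonGameMode to add a new tile, increment score and increase speed.
; The tile then destroys itself after a short delay.
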(event OnComponentBeginOverlap(Box)
  (params (OverlappedComponent :type Primitive%20Component%20Object%20Reference) (OtherActor :type Actor%20Object%20Reference) (OtherComp :type Primitive%20Component%20Object%20Reference) (OtherBodyIndex :type Integer) (bFromSweep :type Boolean) (SweepResult :type Hit%20Result%20Structure%20%28by%20ref%29))
  (bind _asthird_person_game_mode (Utilities|Casting|CastToThirdPersonGameMode (Game|GetGameMode)))
  (Default|AddNewFloorTile _asthird_person_game_mode)
  ;[1 1 1] Increment score by "score multiplier"
  (Default|IncrementScore _asthird_person_game_mode)
  ;[1 1 1] Increment speed
  (Default|IncreaseSpeed _asthird_person_game_mode)
  ;[1 1 1] Delete tile after 2 seconds
  (Utilities|FlowControl|Delay 2.0)
  (Actor|DestroyActor))

(event EventBeginPlay
  (CallFunction|SpawnObstacles))

(event Collision|EventActorBeginOverlap
  (params (OtherActor :type Actor%20Object%20Reference)))

(event EventTick
  (params (DeltaSeconds :type Float%20%28single-precision%29)))

(fn ConstructionScript)

(fn SpawnObstacles
  (bind _newparam (CallFunction|GetRandomLocation))
  (Game|SpawnActorfromClass "/Game/Custom/BluePrints/Obstacles/Block.Block_C" _newparam "Undefined" 0 0))

(fn GetRandomLocation
  (switch int (Math|Random|RandomIntegerinRange 0 2)
    (:0
      (return (Transformation|GetWorldTransform (Variables|Default|GetLane1))))
    (:1
      (return (Transformation|GetWorldTransform (Variables|Default|GetLane2))))
    (:2
      (return (Transformation|GetWorldTransform (Variables|Default|GetLane3))))))